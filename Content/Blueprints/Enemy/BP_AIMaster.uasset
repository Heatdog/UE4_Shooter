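; BP_AIMaster is an enemy AI character with health, damage, random wandering and target sensing.
; A looping timer moves it to random navigable points, while AI Perception passes sensed actors to BP_AiController, clearing them through a delayed timer after sight or sense is lost.
; Damage events reduce health, with a headshot multiplier.
; A polling timer detects negative health, then triggers ragdoll and delayed destruction.
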(event OnPerceptionUpdated(AIPerception)
  (params (UpdatedActors :type Array%20of%20Actor%20Object%20References)))

(event OnTargetPerceptionUpdated(AIPerception)
  (params (Actor :type Actor%20Object%20Reference) (Stimulus :type AI%20Stimulus%20Structure))
  (Variables|Default|SetSenceActor Actor)
  (if (Utilities|Struct|BreakAIStimulus Stimulus)
    (Utilities|Time|ClearandInvalidateTimerbyHandle (Variables|Default|GetLostTimer))
    (Default|SetTargetActor (.AsBP%20Ai%20Controller (Utilities|Casting|CastToBP_AiController (Pawn|GetController))) (Variables|Default|GetSenceActor))
    (else
      (bind _returnvalue (Utilities|Time|SetTimerbyEvent (delegate Custom|TargetLost) 5.0))
      (Variables|Default|SetLostTimer _returnvalue))))

(event Custom|RandomLocation
  (AI|Navigation|SimpleMovetoLocation (Pawn|GetController) (.RandomLocation (Class|NavigationSystemV1|GetRandomPointinNavigableRadius (Transformation|GetActorLocation) 3e+04 0 0))))

(event Custom|EventDestroy
  (params (Dealy :type Float%20%28single-precision%29) (Target :type Actor%20Object%20Reference))
  (Utilities|DestroyMacro Dealy Target))

(event Custom|TargetLost
  (Variables|Default|SetSenceActor 0)
  (Default|SetTargetActor (.AsBP%20Ai%20Controller (Utilities|Casting|CastToBP_AiController (Pawn|GetController))) (Variables|Default|GetSenceActor)))

(event Game|Damage|EventRadialDamage
  (params (DamageReceived :type Float%20%28single-precision%29) (DamageType :type Damage%20Type%20Object%20Reference) (Origin :type Vector :default "0, 0, 0") (HitInfo :type Hit%20Result%20Structure%20%28by%20ref%29) (InstigatedBy :type Controller%20Object%20Reference) (DamageCauser :type Actor%20Object%20Reference))
  (CallFunction|CalculateDamage "None" DamageReceived))

(event EventBeginPlay
  (CallFunction|SetHealth)
  (Utilities|Time|SetTimerbyEvent (delegate Custom|RandomLocation) (Math|Random|RandomFloatinRange 1.0 2.0) true))

(event EventTakingDamage
  (params (Bone :type Name :default "None") (Damage :type Float%20%28single-precision%29) (Instigator :type Actor%20Object%20Reference))
  (CallFunction|CalculateDamage Bone Damage Instigator))

(fn ConstructionScript)

(fn SetHealth
  (Variables|Default|SetcurrentHealth (Variables|Default|GetmaxHealth))
  (bind _returnvalue (Utilities|Time|SetTimerbyFunctionName 0 "Death" 0.1 true))
  (Variables|Default|Settimer _returnvalue))

(fn Death
  (bind _mesh (Variables|Character|GetMesh))
  (if (< (Variables|Default|GetcurrentHealth) 0.0)
    (Class|SkeletalMeshComponent|SetAllBodiesSimulatePhysics _mesh true)
    (Collision|SetCollisionProfileName _mesh "Ragdoll" true :!class /Script/Engine.PrimitiveComponent)
    (Collision|SetCollisionEnabled (Variables|Collision|GetCapsuleComponent) "NoCollision")
    (Utilities|Time|PauseTimerbyHandle (Variables|Default|Gettimer))
    (CallFunction|EventDestroy (LocalVariables|GetTimeDealy) self)))

(fn CalculateDamage
  (params (Bone :type Name) (Damage :type Float%20%28single-precision%29) (Instigator :type Actor%20Object%20Reference))
  (LocalVariables|SetDamageLoc Damage)
  (if (Utilities|Name|Equal(Name) Bone "head")
    (Variables|Default|SetcurrentHealth (- (Variables|Default|GetcurrentHealth) (* (LocalVariables|GetDamageLoc) (LocalVariables|GetDamageMulty))))
    (else
      (Variables|Default|SetcurrentHealth (- (Variables|Default|GetcurrentHealth) (LocalVariables|GetDamageLoc))))))