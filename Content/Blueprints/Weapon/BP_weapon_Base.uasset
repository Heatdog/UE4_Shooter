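; Base weapon Blueprint with single, burst and auto fire, loading its stats from a DT_WEapon row at construction.
; FirePress gates shots on reload and fire-rate flags, looping through a retriggerable delay for burst and auto.
; Each shot traces from the active camera, aims the muzzle at that point, adds random spray, spawns BP_Bullet and applies recoil.
; An empty magazine triggers montage-timed auto-reload; ReloadWeapon separately transfers reserve ammo within WeaponData.
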(event Custom|ChangeFireMode
  (if (not (.SingleType (Utilities|Struct|BreakStruct_weaponData (Variables|Default|GetWeaponData))))
    (switch Utilities|FlowControl|Switch|SwitchonEnum_FireMode (Variables|Default|GetFire%20Mode)
      (:NewEnumerator0
        (Variables|Default|SetFire%20Mode "NewEnumerator2"))
      (:NewEnumerator2
        (Variables|Default|SetFire%20Mode "NewEnumerator0")))))

(event Custom|Fire%20Press
  (params (Trigger%20Pulled :type Boolean))
  ;[1 1 1] Тест Стрельбы
  (Variables|Default|SetFiring Trigger%20Pulled)
  (switch Utilities|FlowControl|Switch|SwitchonEnum_FireMode (Variables|Default|GetFire%20Mode)
    (:NewEnumerator0
      (if (CallFunction|CanShoot)
        (Variables|Default|SetFireRateDelay true)
        (CallFunction|SpawnProjectile)
        (Utilities|FlowControl|RetriggerableDelay (Variables|Default|GetFire%20Rate))
        (Variables|Default|SetFireRateDelay false)
        (Variables|Default|SetFiring false)))
    (:NewEnumerator1
      (if (CallFunction|CanShoot)
        (if (> (.BulletsInBurst (Utilities|Struct|BreakStruct_weaponData (Variables|Default|GetWeaponData))) (Variables|Default|GetCurrentBulletsInBurst)) :!label _label
          (Variables|Default|SetFireRateDelay true)
          (Math|Integer|IncrementInt (Variables|Default|GetCurrentBulletsInBurst)
            (:%20%20
              (CallFunction|SpawnProjectile)
              (Utilities|FlowControl|RetriggerableDelay (Variables|Default|GetFire%20Rate))
              (Variables|Default|SetFireRateDelay false)
              (goto _label)))
          (else
            (Variables|Default|SetCurrentBulletsInBurst 0)
            (Variables|Default|SetFiring false)))))
    (:NewEnumerator2
      (if (CallFunction|CanShoot) :!label _label_2
        (Variables|Default|SetFireRateDelay true)
        (CallFunction|SpawnProjectile)
        (Utilities|FlowControl|RetriggerableDelay (Variables|Default|GetFire%20Rate))
        (Variables|Default|SetFireRateDelay false)
        (goto _label_2)))))

(event Custom|AutoReload
  (bind _weapondata (Variables|Default|GetWeaponData))
  (bind _weapondata_2 (Variables|Default|GetWeaponData))
  (bind (_reloaddelay _reloadmontage) (Utilities|Struct|BreakStruct_weaponData _weapondata_2))
  (bind (_ammomax _ammoinclip _ammocurrent) (Utilities|Struct|BreakStruct_weaponData _weapondata))
  ;[1 1 1] Отжали кнопку - автоматическая перезарядка
  (if (== _ammocurrent 0)
    (if (not (== _ammomax 0))
      (Variables|Default|SetIsReloading true)
      (CallFunction|Reloading)
      (CallFunction|PlayMontage _reloadmontage "/Game/TestAnim/Reload_Rifle_Hip_Montage.Reload_Rifle_Hip_Montage")
      (Utilities|FlowControl|Delay _reloaddelay)
      (Variables|Default|SetIsReloading false))))

(event Custom|ReloadWeapon
  ;[1 1 1] Перезарядка оружия
  (if (> (.AmmoMax (Utilities|Struct|BreakStruct_weaponData (Variables|Default|GetWeaponData))) 0)
    (Variables|Default|SetNeededAmmo (- (.AmmoInClip (Utilities|Struct|BreakStruct_weaponData (Variables|Default|GetWeaponData))) (.AmmoCurrent (Utilities|Struct|BreakStruct_weaponData (Variables|Default|GetWeaponData)))))
    (if (<= (.AmmoMax (Utilities|Struct|BreakStruct_weaponData (Variables|Default|GetWeaponData))) (Variables|Default|GetNeededAmmo))
      (Variables|Default|SetWeaponData (Utilities|Struct|MakeStruct_weaponData (.FireMode (Utilities|Struct|BreakStruct_weaponData (Variables|Default|GetWeaponData))) (.MuzzleName (Utilities|Struct|BreakStruct_weaponData (Variables|Default|GetWeaponData))) (.FireRate (Utilities|Struct|BreakStruct_weaponData (Variables|Default|GetWeaponData))) (.reloadDelay (Utilities|Struct|BreakStruct_weaponData (Variables|Default|GetWeaponData))) (.WeaponSpray (Utilities|Struct|BreakStruct_weaponData (Variables|Default|GetWeaponData))) (.DamageMin (Utilities|Struct|BreakStruct_weaponData (Variables|Default|GetWeaponData))) (.DamageMax (Utilities|Struct|BreakStruct_weaponData (Variables|Default|GetWeaponData))) 0 (.AmmoInClip (Utilities|Struct|BreakStruct_weaponData (Variables|Default|GetWeaponData))) (+ (.AmmoMax (Utilities|Struct|BreakStruct_weaponData (Variables|Default|GetWeaponData))) (.AmmoCurrent (Utilities|Struct|BreakStruct_weaponData (Variables|Default|GetWeaponData)))) (.FiringMontage (Utilities|Struct|BreakStruct_weaponData (Variables|Default|GetWeaponData))) (.ReloadMontage (Utilities|Struct|BreakStruct_weaponData (Variables|Default|GetWeaponData))) (.WeaponRecoil (Utilities|Struct|BreakStruct_weaponData (Variables|Default|GetWeaponData))) (.BulletsInBurst (Utilities|Struct|BreakStruct_weaponData (Variables|Default|GetWeaponData))) (.SingleType (Utilities|Struct|BreakStruct_weaponData (Variables|Default|GetWeaponData)))))
      (else
        (Variables|Default|SetWeaponData (Utilities|Struct|MakeStruct_weaponData (.FireMode (Utilities|Struct|BreakStruct_weaponData (Variables|Default|GetWeaponData))) (.MuzzleName (Utilities|Struct|BreakStruct_weaponData (Variables|Default|GetWeaponData))) (.FireRate (Utilities|Struct|BreakStruct_weaponData (Variables|Default|GetWeaponData))) (.reloadDelay (Utilities|Struct|BreakStruct_weaponData (Variables|Default|GetWeaponData))) (.WeaponSpray (Utilities|Struct|BreakStruct_weaponData (Variables|Default|GetWeaponData))) (.DamageMin (Utilities|Struct|BreakStruct_weaponData (Variables|Default|GetWeaponData))) (.DamageMax (Utilities|Struct|BreakStruct_weaponData (Variables|Default|GetWeaponData))) (- (.AmmoMax (Utilities|Struct|BreakStruct_weaponData (Variables|Default|GetWeaponData))) (Variables|Default|GetNeededAmmo)) (.AmmoInClip (Utilities|Struct|BreakStruct_weaponData (Variables|Default|GetWeaponData))) (.AmmoInClip (Utilities|Struct|BreakStruct_weaponData (Variables|Default|GetWeaponData))) (.FiringMontage (Utilities|Struct|BreakStruct_weaponData (Variables|Default|GetWeaponData))) (.ReloadMontage (Utilities|Struct|BreakStruct_weaponData (Variables|Default|GetWeaponData))) (.WeaponRecoil (Utilities|Struct|BreakStruct_weaponData (Variables|Default|GetWeaponData))) (.BulletsInBurst (Utilities|Struct|BreakStruct_weaponData (Variables|Default|GetWeaponData))) (.SingleType (Utilities|Struct|BreakStruct_weaponData (Variables|Default|GetWeaponData)))))))))

(event Custom|Reloading
  (bind _weapondata (Variables|Default|GetWeaponData))
  (bind _weapondata_2 (Variables|Default|GetWeaponData))
  (bind (_reloaddelay _reloadmontage) (Utilities|Struct|BreakStruct_weaponData _weapondata_2))
  (bind (_ammomax _ammoinclip _ammocurrent) (Utilities|Struct|BreakStruct_weaponData _weapondata))
  ;[1 1 1] ручная перезарядка
  (if (not (== _ammomax 0))
    (if (not (== _ammoinclip _ammocurrent))
      (bind _output_get (Variables|Default|SetIsReloading true))
      (if _output_get
        (CallFunction|PlayMontage _reloadmontage "/Game/TestAnim/Reload_Rifle_Hip_Montage.Reload_Rifle_Hip_Montage")
        (Utilities|FlowControl|Delay _reloaddelay)
        (Variables|Default|SetIsReloading false)))))

(fn ConstructionScript
  ;[1 1 1] Запись в переменные информации с DataTable
  (bind _returnvalue (Utilities|GetDataTableRow "/Game/Blueprints/Weapon/DT_WEapon.DT_WEapon" (Variables|Default|GetWeaponRawnName))
    (:then
      (bind _output_get (Variables|Default|SetWeaponData _returnvalue))
      (Variables|Default|SetFire%20Mode (.FireMode (Utilities|Struct|BreakStruct_weaponData _output_get)))
      (Variables|Default|SetMuzzle%20Name (.MuzzleName (Utilities|Struct|BreakStruct_weaponData _output_get)))
      (Variables|Default|SetFire%20Rate (.FireRate (Utilities|Struct|BreakStruct_weaponData _output_get)))
      (Variables|Default|SetReload%20Delay (.reloadDelay (Utilities|Struct|BreakStruct_weaponData _output_get)))
      (Variables|Default|SetWeapon%20Spray (.WeaponSpray (Utilities|Struct|BreakStruct_weaponData _output_get)))
      (Variables|Default|SetOneHand (.OneHand (Utilities|Struct|BreakStruct_weaponData _output_get))))))

(fn CalculateDirection
  (bind _returnvalue (Utilities|MuzzlePosition))
  (bind _charref (Variables|Default|GetCharRef))
  (bind _weaponcamera (Variables|Default|GetWeaponCamera))
  (bind _fcamera (Variables|/Game/Blueprints/Player/BPPlayerCharacter.BPPlayerCharacter_C|GetFCamera _charref))
  (bind _aiming (Variables|/Game/Blueprints/Player/BPPlayerCharacter.BPPlayerCharacter_C|GetAiming _charref))
  (bind _returnvalue_2 (select _aiming _weaponcamera _fcamera))
  (bind _returnvalue_3 (Transformation|GetWorldTransform _returnvalue_2))
  (bind _end (|EndPoint (.rotation _returnvalue_3) (.location _returnvalue_3)))
  ;[1 1 1] Настройка камеры прицеливания
  ;[1 1 1] Рассчет дальности стрельбы
  (bind (_outhit _returnvalue_4) (Collision|LineTraceForObjects (|StartPoint (.rotation _returnvalue_3) (.location _returnvalue_3)) _end (Utilities|Array|MakeArray "ObjectTypeQuery1") false 0 "ForDuration" true "(R=1.000000,G=0.000000,B=0.000000,A=1.000000)" "(R=0.000000,G=1.000000,B=0.000000,A=1.000000)" 0.0))
  (return _returnvalue (Math|Rotator|FindLookatRotation _returnvalue (Math|Vector|SelectVector (.ImpactPoint (Collision|BreakHitResult _outhit)) _end _returnvalue_4))))

(fn SpawnProjectile
  (if (CallFunction|HasAmmoinMag)
    ;[1 1 1] Анимация затвора
    (if (Variables|Default|GetOneHand)
      (CallFunction|PlayMontage (.FiringMontage (Utilities|Struct|BreakStruct_weaponData (Variables|Default|GetWeaponData))) "/Game/TestAnim/Idle_Pistol_Montage.Idle_Pistol_Montage")
      (else
        (CallFunction|PlayMontage (.FiringMontage (Utilities|Struct|BreakStruct_weaponData (Variables|Default|GetWeaponData))) (select (Variables|/Game/Blueprints/Player/BPPlayerCharacter.BPPlayerCharacter_C|GetAiming (Variables|Default|GetCharRef)) "/Game/TestAnim/Fire_Rifle_Ironsights_Montage.Fire_Rifle_Ironsights_Montage" "/Game/TestAnim/Fire_Rifle_Hip_Montage.Fire_Rifle_Hip_Montage"))))
    (bind (_location _rotation) (CallFunction|CalculateDirection))
    ;[1 1 1] Рассчет стрельбы с спреем
    (bind _transform (CallFunction|CalculateFinalDirection _location _rotation))
    (Game|SpawnActorfromClass "/Game/Blueprints/Weapon/BP_bullet.BP_Bullet_C" _transform "Undefined" 0 (Math|Random|RandomFloatinRange (.DamageMin (Utilities|Struct|BreakStruct_weaponData (Variables|Default|GetWeaponData))) (.DamageMax (Utilities|Struct|BreakStruct_weaponData (Variables|Default|GetWeaponData)))) 0)
    (Default|WeaponRecoil (Variables|Default|GetCharRef) (.WeaponRecoil (Utilities|Struct|BreakStruct_weaponData (Variables|Default|GetWeaponData))))
    (Variables|Default|SetWeaponData (Utilities|Struct|MakeStruct_weaponData (.FireMode (Utilities|Struct|BreakStruct_weaponData (Variables|Default|GetWeaponData))) (.MuzzleName (Utilities|Struct|BreakStruct_weaponData (Variables|Default|GetWeaponData))) (.FireRate (Utilities|Struct|BreakStruct_weaponData (Variables|Default|GetWeaponData))) (.reloadDelay (Utilities|Struct|BreakStruct_weaponData (Variables|Default|GetWeaponData))) (.WeaponSpray (Utilities|Struct|BreakStruct_weaponData (Variables|Default|GetWeaponData))) (.DamageMin (Utilities|Struct|BreakStruct_weaponData (Variables|Default|GetWeaponData))) (.DamageMax (Utilities|Struct|BreakStruct_weaponData (Variables|Default|GetWeaponData))) (.AmmoMax (Utilities|Struct|BreakStruct_weaponData (Variables|Default|GetWeaponData))) (.AmmoInClip (Utilities|Struct|BreakStruct_weaponData (Variables|Default|GetWeaponData))) (- (.AmmoCurrent (Utilities|Struct|BreakStruct_weaponData (Variables|Default|GetWeaponData))) 1) (.FiringMontage (Utilities|Struct|BreakStruct_weaponData (Variables|Default|GetWeaponData))) (.ReloadMontage (Utilities|Struct|BreakStruct_weaponData (Variables|Default|GetWeaponData))) (.WeaponRecoil (Utilities|Struct|BreakStruct_weaponData (Variables|Default|GetWeaponData))) (.BulletsInBurst (Utilities|Struct|BreakStruct_weaponData (Variables|Default|GetWeaponData))) (.SingleType (Utilities|Struct|BreakStruct_weaponData (Variables|Default|GetWeaponData)))))
    (else
      (CallFunction|AutoReload))))

(fn CalculateFinalDirection
  (params (Location :type Vector) (Rotation :type Rotator))
  (bind _weapon_spray (Variables|Default|GetWeapon%20Spray))
  (bind _returnvalue (* -1 _weapon_spray))
  (return (Math|Transform|MakeTransform Location (Math|Rotator|CombineRotators Rotation (Math|Rotator|MakeRotator (Math|Random|RandomFloatinRange _returnvalue 0.0) (Math|Random|RandomFloatinRange _returnvalue 0.0) (Math|Random|RandomFloatinRange _returnvalue 0.0))))))

(fn PlayMontage
  (params (WeaponAnim :type Anim%20Montage%20Object%20Reference) (CharAnim :type Anim%20Montage%20Object%20Reference))
  (Animation|Montage|MontagePlay (Components|SkeletalMesh|GetAnimInstance (Variables|Default|GetWeaponMesh)) WeaponAnim 1.0 "MontageLength" 0.0 true)
  (Animation|Montage|MontagePlay (Components|SkeletalMesh|GetAnimInstance (Variables|/Script/Engine.Character|GetMesh (Variables|Default|GetCharRef))) CharAnim 1.0 "MontageLength" 0.0 true))

(fn HasAmmoinMag
  (return (> (.AmmoCurrent (Utilities|Struct|BreakStruct_weaponData (Variables|Default|GetWeaponData))) 0)))

(fn CanShoot
  (return (Math|Boolean|ANDBoolean (Variables|Default|GetFiring) (not (Variables|Default|GetIsReloading)) (not (Variables|Default|GetFireRateDelay)))))