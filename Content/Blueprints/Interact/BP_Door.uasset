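; Door actor that reacts to the Interact event inherited from its parent class.
; Each interaction calls the parent logic, then adds a 90-degree local rotation to the static mesh instantly, with no open/closed state or animation.
; For Hold-type interactions, it then rebuilds InteractData, copying name, availability and duration but not passing Type through.
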(event EventBeginPlay)

(event Collision|EventActorBeginOverlap
  (params (OtherActor :type Actor%20Object%20Reference)))

(event EventTick
  (params (DeltaSeconds :type Float%20%28single-precision%29))
  (|CallParentFunction DeltaSeconds) ; This node is disabled and will not be called.\nDrag off pins to build functionality.
)

(event EventInteract
  (|CallParentFunction)
  (Transformation|AddLocalRotation (Variables|Default|GetStaticMesh) "0,90.000000, 0" false false)
  (switch Utilities|FlowControl|Switch|SwitchonEnum_Interact (.Type (Utilities|Struct|BreakStruct_Interact (Variables|Default|GetInteractData)))
    (:NewEnumerator1
      (Variables|Default|SetInteractData (Utilities|Struct|MakeStruct_Interact (.Name (Utilities|Struct|BreakStruct_Interact (Variables|Default|GetInteractData))) "NewEnumerator0" (.IsAvaiable (Utilities|Struct|BreakStruct_Interact (Variables|Default|GetInteractData))) (.TimeDuration (Utilities|Struct|BreakStruct_Interact (Variables|Default|GetInteractData))))))))

(fn ConstructionScript
  (|CallParentFunction))