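; Base pickup actor that shows a floating name label when the player character is nearby.
; Tick checks the distance to the player pawn against a fixed radius and calls ShowName or HideName to toggle the widget component.
; ShowName lazily creates the name widget once from InteractData's Name field.
; Interact only sets a flag, and CheckInvability is an empty event.
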(event Custom|Interact
  (Variables|Default|SetIntearct true))

(event Custom|CheckInvability)

(event Custom|ShowName
  (bind _widget (Variables|Default|GetWidget))
  (Utilities|IsValid (Variables|Default|GetWD_Name)
    (:Is%20Valid
      _)
    (:Is%20Not%20Valid
      (bind _returnvalue (UserInterface|CreateWidget "/Game/UMG/WD_PickupName.WD_PickupName_C" 0 (.Name (Utilities|Struct|BreakStruct_Interact (Variables|Default|GetInteractData)))))
      (bind _output_get (Variables|Default|SetWD_Name _returnvalue))
      (UserInterface|SetWidget _widget _output_get)))
  (Rendering|SetVisibility _widget true false))

(event Custom|HideName
  (Rendering|SetVisibility (Variables|Default|GetWidget) false false))

(event EventTick
  (params (DeltaSeconds :type Float%20%28single-precision%29))
  (bind _asbpplayer_character (Utilities|Casting|CastToBPPlayerCharacter (Game|Player|GetPlayerPawn 0)))
  (if (< (Math|Vector|Distance(Vector) (Transformation|GetActorLocation _asbpplayer_character) (Transformation|GetActorLocation)) 2e+02)
    (CallFunction|ShowName)
    (else
      (CallFunction|HideName))))

(fn ConstructionScript)