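; AI controller Blueprint that runs a behavior tree on possession and feeds it player detection from AI perception.
; On each perception update for a BPPlayerCharacter tagged Player, it writes whether the stimulus was sensed to the SeePlayer blackboard key.
; It also switches the AI_State enum key between two values based on that result.
; Updates for actors failing the character cast only print a red debug string.
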(event OnTargetPerceptionUpdated(AIPerception)
  (params (Actor :type Actor%20Object%20Reference) (Stimulus :type AI%20Stimulus%20Structure))
  (bind _bsuccessfullysensed (Utilities|Struct|BreakAIStimulus Stimulus))
  (bind _returnvalue (AI|GetBlackboard 0))
  (bind _asbpplayer_character (Utilities|Casting|CastToBPPlayerCharacter Actor)
    (:then
      (if (Utilities|Name|Equal(Name) (Variables|/Game/Blueprints/Player/BPPlayerCharacter.BPPlayerCharacter_C|GetTag _asbpplayer_character) "Player")
        (AI|Components|Blackboard|SetValueasBool _returnvalue (Utilities|Name|MakeLiteralName "SeePlayer") _bsuccessfullysensed)
        (if _bsuccessfullysensed
          (AI|Components|Blackboard|SetValueasEnum _returnvalue (Utilities|Name|MakeLiteralName "AI_State") 1)
          (else
            (AI|Components|Blackboard|SetValueasEnum _returnvalue (Utilities|Name|MakeLiteralName "AI_State"))))))
    (:CastFailed
      (Development|PrintString "LLLL" true true "(R=1.000000,G=0.000000,B=0.023145,A=1.000000)"))))

(event EventBeginPlay)

(event EventTick
  (params (DeltaSeconds :type Float%20%28single-precision%29)))

(event EventPossess
  (params (PossessedPawn :type Pawn%20Object%20Reference))
  (AI|RunBehaviorTree))

(fn ConstructionScript)